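; BP_DDAAGun is a prop, apparently an AA gun, whose base rotation is driven by a physics-based controller component.
; Each Tick teleports ControllerZAxis using ControllerSupport's world X/Y and its own world Z, passed as a relative location with default rotation.
; It then prints the controller's angular velocity and adds it to BaseAoR as a velocity-change angular impulse, so spin accumulates rather than being matched.
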(event `self.ReceiveTick`
  (params (DeltaSeconds :type "Float (single-precision)"))
  (bind _controller_zaxis (`self.Controller-ZAxis`))
  (`|ExecutionSequence`
    (:`then_0`
      (`SceneComponent.K2_SetRelativeLocationAndRotation` :`self` _controller_zaxis :`NewLocation` (`KismetMathLibrary.MakeVector` (.x (`SceneComponent.K2_GetComponentLocation` (`self.Controller-Support`))) (.y (`SceneComponent.K2_GetComponentLocation` (`self.Controller-Support`))) (.z (`SceneComponent.K2_GetComponentLocation` _controller_zaxis))) :`bTeleport` true))
    (:`then_1`
      (bind _returnvalue (`PrimitiveComponent.GetPhysicsAngularVelocity` (`self.Controller-ZAxis`) "None"))
      (`KismetSystemLibrary.PrintString` (`KismetStringLibrary.Conv_VectorToString` _returnvalue))
      (`PrimitiveComponent.AddAngularImpulse` (`self.Base-AoR`) _returnvalue "None" true))))

(fn `UserConstructionScript`)